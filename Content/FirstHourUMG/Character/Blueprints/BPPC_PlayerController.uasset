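; Player controller for the FirstHourUMG game that toggles a pause menu on the Pause input.
; When no menu exists, it creates WBP_MainMenu, shows it with Game and UI input and mouse cursor, pauses the game and hides the character's HUD.
; When the menu is open, it removes and clears it, restores game-only input, hides the cursor, unpauses and shows the HUD again.
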(event EventBeginPlay)

(event EventTick
  (params (DeltaSeconds :type Float%20%28single-precision%29)))

(event Input|ActionEvents|InputActionPause
  (params (Key :type Key%20Structure :default "None"))
  (bind _returnvalue (Game|GetPlayerCharacter 0))
  (:Pressed
    (Utilities|IsValid (Variables|Default|GetPauseMenu)
      (:Is%20Valid
        (Input|SetInputModeGameOnly self)
        (Game|SetGamePaused false)
        (Variables|Default|SetbShowMouseCursor false)
        (Widget|RemovefromParent (Variables|Default|GetPauseMenu))
        (Variables|Default|SetPauseMenu 0)
        (bind _ascharacter_first_hour_umg (Utilities|Casting|CastToCharacter_FirstHourUMG _returnvalue))
        (Default|ShowHUD _ascharacter_first_hour_umg))
      (:Is%20Not%20Valid
        (bind _returnvalue_2 (UserInterface|CreateWidget "/Game/FirstHourUMG/Widgets/WBP_MainMenu.WBP_MainMenu_C"))
        (Variables|Default|SetPauseMenu _returnvalue_2)
        (UserInterface|Viewport|AddtoViewport _returnvalue_2 0)
        (Input|SetInputModeGameandUI self 0 "DoNotLock" true)
        (Variables|Default|SetbShowMouseCursor true)
        (Game|SetGamePaused true)
        (bind _ascharacter_first_hour_umg_2 (Utilities|Casting|CastToCharacter_FirstHourUMG _returnvalue))
        (Default|HideHUD _ascharacter_first_hour_umg_2)))))

(fn ConstructionScript)