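; GM_FirstHourUMG is a game mode Blueprint that handles the win and game over end states.
; HandleGameWin and HandleGameOver follow the same sequence, showing WBP_WinScreen or WBP_GameOver respectively.
; Each switches to UI-only input with a visible, unlocked cursor, adds its widget to the viewport and pauses the game.
; Both then cast the player character to Character_Main to hide its HUD.
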(event Custom|Handle%20Game%20Win
  (bind _returnvalue (Game|GetPlayerController 0))
  (Input|SetInputModeUIOnly _returnvalue 0 "DoNotLock")
  (bind _returnvalue_2 (UserInterface|CreateWidget "/Game/FirstHourUMG/Widgets/WBP_WinScreen.WBP_WinScreen_C"))
  (Variables|/Script/Engine.PlayerController|SetbShowMouseCursor _returnvalue true)
  (UserInterface|Viewport|AddtoViewport _returnvalue_2 0)
  (Game|SetGamePaused true)
  (bind _ascharacter_first_hour_umg (Utilities|Casting|CastToCharacter_Main (Game|GetPlayerCharacter 0)))
  (Default|HideHUD _ascharacter_first_hour_umg))

(event Custom|Handle%20Game%20Over
  (bind _returnvalue (Game|GetPlayerController 0))
  (Input|SetInputModeUIOnly _returnvalue 0 "DoNotLock")
  (bind _returnvalue_2 (UserInterface|CreateWidget "/Game/FirstHourUMG/Widgets/WBP_GameOver.WBP_GameOver_C"))
  (Variables|/Script/Engine.PlayerController|SetbShowMouseCursor _returnvalue true)
  (UserInterface|Viewport|AddtoViewport _returnvalue_2 0)
  (Game|SetGamePaused true)
  (bind _ascharacter_first_hour_umg (Utilities|Casting|CastToCharacter_Main (Game|GetPlayerCharacter 0)))
  (Default|HideHUD _ascharacter_first_hour_umg))

(fn ConstructionScript)